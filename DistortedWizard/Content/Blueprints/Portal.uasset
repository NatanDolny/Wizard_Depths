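; Portal actor that spins around its roll axis and teleports the ThirdPersonCharacter to a linked Target portal.
; On box overlap, if Portable, it clears the target's Portable flag, waits briefly, then calls PortalTo with the target box's location and the player's control rotation.
; Nothing in this file re-enables Portable.
; The construction script builds a dynamic orange portal material and passes PortalImage to an unnamed texture parameter.
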(event `self.ReceiveTick`
  (params (DeltaSeconds :type "Float (single-precision)"))
  (`self.K2_AddActorLocalRotation` (`KismetMathLibrary.MakeRotator` (* DeltaSeconds 100.0))))

(event `self.Box.OnComponentBeginOverlap`
  (params (OverlappedComponent :type "PrimitiveComponent Object Reference") (OtherActor :type "Actor Object Reference") (OtherComp :type "PrimitiveComponent Object Reference") (OtherBodyIndex :type Integer) (bFromSweep :type Boolean) (SweepResult :type "HitResult Structure (by ref)"))
  (bind _target (`self.Target`))
  (bind _asthird_person_character (cast `/Game/ThirdPersonBP/Blueprints/ThirdPersonCharacter` OtherActor))
  (set `self.As Third Person Character` _asthird_person_character)
  (if (`self.Portable`)
    (set `/Game/Blueprints/Portal.Portable` false _target)
    (`KismetSystemLibrary.Delay` 0.05)
    (`/Game/ThirdPersonBP/Blueprints/ThirdPersonCharacter.PortalTo` (`self.As Third Person Character`) (`SceneComponent.K2_GetComponentLocation` (`/Game/Blueprints/Portal.Box` _target)) (`Controller.GetControlRotation` (`GameplayStatics.GetPlayerController` 0)))))

(fn `UserConstructionScript`
  (bind _portalmesh (`self.PortalMesh`))
  (bind _returnvalue (`PrimitiveComponent.CreateDynamicMaterialInstance` _portalmesh 0 "/Game/Textures/OrangePortal_Mat.OrangePortal_Mat" "None"))
  (`MaterialInstanceDynamic.SetTextureParameterValue` _returnvalue "None" (`self.PortalImage`))
  (`PrimitiveComponent.SetMaterial` _portalmesh 0 _returnvalue))