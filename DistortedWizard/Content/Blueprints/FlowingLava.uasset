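; FlowingLava is a lava actor that switches its Lava component between a molten and a cooled look.
; Every Tick it reads the Frozen flag, applying the cooled material with shadow casting when true and the molten material without shadows otherwise.
; Nothing in this Blueprint sets Frozen, and a leftover visibility-toggle branch is disconnected and never runs.
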(event `self.ReceiveBeginPlay`)

(event `self.ReceiveTick`
  (params (DeltaSeconds :type "Float (single-precision)"))
  (bind _lava (`self.Lava`))
  (bind _lava_2 (`self.Lava`))
  (`|ExecutionSequence`
    (:`then_0`
      (if (`self.Frozen`)
        (`PrimitiveComponent.SetMaterial` _lava 0 "/Game/InfinityBladeFireLands/Environments/Fire/Env_Fire_Terrain2/Materials/M_Cooled_Lava_Inst.M_Cooled_Lava_Inst")
        (`PrimitiveComponent.SetCastShadow` _lava_2 true)
        (else
          (`PrimitiveComponent.SetMaterial` _lava 0 "/Game/InfinityBladeFireLands/Environments/Fire/Env_Fire_FlameDungeon/Materials/M_Dungeon_Pipes_Lava.M_Dungeon_Pipes_Lava")
          (`PrimitiveComponent.SetCastShadow` _lava_2 false))))))

(fn `UserConstructionScript`)