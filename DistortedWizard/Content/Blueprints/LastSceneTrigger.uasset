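; LastSceneTrigger is a trigger actor that starts what its names indicate is the game's last scene.
; The first overlap of its Box component, by any actor, creates players for the LastScene and LastSequence level sequences and plays both back to back without waiting.
; BeginPlay casts the player character to ThirdPersonCharacter but sets PlayerReference to None, and the overlap logic never uses it.
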(event `self.ReceiveBeginPlay`
  (bind _asthird_person_character (cast `/Game/ThirdPersonBP/Blueprints/ThirdPersonCharacter` (`GameplayStatics.GetPlayerCharacter` 0)))
  (set `self.PlayerReference` null))

(event `self.Box.OnComponentBeginOverlap`
  (params (OverlappedComponent :type "PrimitiveComponent Object Reference") (OtherActor :type "Actor Object Reference") (OtherComp :type "PrimitiveComponent Object Reference") (OtherBodyIndex :type Integer) (bFromSweep :type Boolean) (SweepResult :type "HitResult Structure (by ref)"))
  (`/Engine/EditorBlueprintResources/StandardMacros.DoOnce` false
    (:`Completed`
      (bind (_outactor _returnvalue) (`LevelSequencePlayer.CreateLevelSequencePlayer` "/Game/Animations/LastScene.LastScene"))
      (bind _output_get (set `self.LastScene` _returnvalue))
      (`MovieSceneSequencePlayer.Play` _output_get)
      (bind (_outactor_2 _returnvalue_2) (`LevelSequencePlayer.CreateLevelSequencePlayer` "/Game/Animations/LastSequence.LastSequence"))
      (bind _output_get_2 (set `self.LastSequence` _returnvalue_2))
      (`MovieSceneSequencePlayer.Play` _output_get_2))))

(fn `UserConstructionScript`)